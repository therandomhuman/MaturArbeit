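; Anim notify that plays surface-dependent footstep sounds for the animated mesh's owner.
; It traces from the actor's location along its negative up vector on the Visibility channel and switches on the hit's physical surface type.
; Each terrain surface picks a random sound from SoundDataAsset and plays it at the actor's location with master volume and random pitch.
; All surfaces apply the attenuation settings except Layer 05.
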(fn ReceivedNotify
  (params (MeshComp :type Skeletal%20Mesh%20Component%20Object%20Reference) (Animation :type Anim%20Sequence%20Base%20Object%20Reference) (EventReference :type Anim%20Notify%20Event%20Reference%20Structure%20%28by%20ref%29))
  (bind _returnvalue (Components|GetOwner MeshComp))
  (bind _sounddataasset (Variables|Default|GetSoundDataAsset))
  (bind _returnvalue_2 (Transformation|GetActorLocation _returnvalue))
  (bind _footstep_sounds (Variables|/Game/AzielArts_Material/Footsteps/Blueprints/BP_Footsteps.BP_Footsteps_C|GetFootstep%20Sounds _sounddataasset))
  (bind (_snow _puddleice _beach _layer01 _layer01_slope _layer02 _layer02_slope _layer03 _layer03_slope _layer04 _layer04_slope _layer05 _layer05_slope _layer06 _layer06_slope) (Utilities|Struct|BreakST_Footsetps _footstep_sounds))
  (LocalVariables|SetFoostepLocation _returnvalue_2)
  (bind (_outhit _returnvalue_3) (Collision|LineTraceByChannel _returnvalue_2 (+ _returnvalue_2 (* (Transformation|GetActorUpVector _returnvalue) -2e+02)) "TraceTypeQuery1" false 0 "None"))
  (if _returnvalue_3
    (LocalVariables|SetRandomPitch (Math|Random|RandomFloatinRange (Variables|Default|GetRandomPitch%20Min) (Variables|Default|GetRandomPitch%20Max)))
    (switch Utilities|FlowControl|Switch|SwitchonEPhysicalSurface (Collision|GetSurfaceType _outhit)
      (:SurfaceType1
        (Audio|PlaySoundatLocation (.OutItem (Utilities|Array|Random _snow)) (LocalVariables|GetFoostepLocation) "0, 0, 0" (Variables|Default|GetMasterVolume) (LocalVariables|GetRandomPitch) 0.0 (Variables|Default|GetAttenuation%20Settings) 0 0 0))
      (:SurfaceType2
        (Audio|PlaySoundatLocation (.OutItem (Utilities|Array|Random _puddleice)) (LocalVariables|GetFoostepLocation) "0, 0, 0" (Variables|Default|GetMasterVolume) (LocalVariables|GetRandomPitch) 0.0 (Variables|Default|GetAttenuation%20Settings) 0 0 0))
      (:SurfaceType3
        (Audio|PlaySoundatLocation (.OutItem (Utilities|Array|Random _beach)) (LocalVariables|GetFoostepLocation) "0, 0, 0" (Variables|Default|GetMasterVolume) (LocalVariables|GetRandomPitch) 0.0 (Variables|Default|GetAttenuation%20Settings) 0 0 0))
      (:SurfaceType4
        (Audio|PlaySoundatLocation (.OutItem (Utilities|Array|Random _layer01)) (LocalVariables|GetFoostepLocation) "0, 0, 0" (Variables|Default|GetMasterVolume) (LocalVariables|GetRandomPitch) 0.0 (Variables|Default|GetAttenuation%20Settings) 0 0 0))
      (:SurfaceType5
        (Audio|PlaySoundatLocation (.OutItem (Utilities|Array|Random _layer01_slope)) (LocalVariables|GetFoostepLocation) "0, 0, 0" (Variables|Default|GetMasterVolume) (LocalVariables|GetRandomPitch) 0.0 (Variables|Default|GetAttenuation%20Settings) 0 0 0))
      (:SurfaceType6
        (Audio|PlaySoundatLocation (.OutItem (Utilities|Array|Random _layer02)) (LocalVariables|GetFoostepLocation) "0, 0, 0" (Variables|Default|GetMasterVolume) (LocalVariables|GetRandomPitch) 0.0 (Variables|Default|GetAttenuation%20Settings) 0 0 0))
      (:SurfaceType7
        (Audio|PlaySoundatLocation (.OutItem (Utilities|Array|Random _layer02_slope)) (LocalVariables|GetFoostepLocation) "0, 0, 0" (Variables|Default|GetMasterVolume) (LocalVariables|GetRandomPitch) 0.0 (Variables|Default|GetAttenuation%20Settings) 0 0 0))
      (:SurfaceType8
        (Audio|PlaySoundatLocation (.OutItem (Utilities|Array|Random _layer03)) (LocalVariables|GetFoostepLocation) "0, 0, 0" (Variables|Default|GetMasterVolume) (LocalVariables|GetRandomPitch) 0.0 (Variables|Default|GetAttenuation%20Settings) 0 0 0))
      (:SurfaceType9
        (Audio|PlaySoundatLocation (.OutItem (Utilities|Array|Random _layer03_slope)) (LocalVariables|GetFoostepLocation) "0, 0, 0" (Variables|Default|GetMasterVolume) (LocalVariables|GetRandomPitch) 0.0 (Variables|Default|GetAttenuation%20Settings) 0 0 0))
      (:SurfaceType10
        (Audio|PlaySoundatLocation (.OutItem (Utilities|Array|Random _layer04)) (LocalVariables|GetFoostepLocation) "0, 0, 0" (Variables|Default|GetMasterVolume) (LocalVariables|GetRandomPitch) 0.0 (Variables|Default|GetAttenuation%20Settings) 0 0 0))
      (:SurfaceType11
        (Audio|PlaySoundatLocation (.OutItem (Utilities|Array|Random _layer04_slope)) (LocalVariables|GetFoostepLocation) "0, 0, 0" (Variables|Default|GetMasterVolume) (LocalVariables|GetRandomPitch) 0.0 (Variables|Default|GetAttenuation%20Settings) 0 0 0))
      (:SurfaceType12
        (Audio|PlaySoundatLocation (.OutItem (Utilities|Array|Random _layer05)) (LocalVariables|GetFoostepLocation) "0, 0, 0" (Variables|Default|GetMasterVolume) (LocalVariables|GetRandomPitch) 0.0 0 0 0 0))
      (:SurfaceType13
        (Audio|PlaySoundatLocation (.OutItem (Utilities|Array|Random _layer05_slope)) (LocalVariables|GetFoostepLocation) "0, 0, 0" (Variables|Default|GetMasterVolume) (LocalVariables|GetRandomPitch) 0.0 (Variables|Default|GetAttenuation%20Settings) 0 0 0))
      (:SurfaceType14
        (Audio|PlaySoundatLocation (.OutItem (Utilities|Array|Random _layer06)) (LocalVariables|GetFoostepLocation) "0, 0, 0" (Variables|Default|GetMasterVolume) (LocalVariables|GetRandomPitch) 0.0 (Variables|Default|GetAttenuation%20Settings) 0 0 0))
      (:SurfaceType15
        (Audio|PlaySoundatLocation (.OutItem (Utilities|Array|Random _layer06_slope)) (LocalVariables|GetFoostepLocation) "0, 0, 0" (Variables|Default|GetMasterVolume) (LocalVariables|GetRandomPitch) 0.0 (Variables|Default|GetAttenuation%20Settings) 0 0 0))))
  (return false))